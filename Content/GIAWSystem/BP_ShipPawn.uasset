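; BP_ShipPawn is a ship pawn Blueprint that adds Konami-style cheat code entry.
; Up, Down, Left, Right, A and B presses append letters to a sequence checked against the Codes array, with a one-second retriggerable delay clearing unmatched input.
; A match plays a secret sound and calls the same-index Cheats function by name through a short timer, allowing cheats such as SpeedCode, which sets ship speed.
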(event `InputAction|Up`
  (params (Key :type "Key Structure"))
  ;[1 1 1] Code Inputs
  (:`Pressed`
    (`self.CheckCode` "u")))

(event `CheckCode`
  (params (Input :type String))
  ;[1 1 1] Check code from array
  (set `self.KonamiCodeSequence` (`KismetStringLibrary.Concat_StrStr` (`self.KonamiCodeSequence`) Input))
  (for (_array_element _array_index) (`self.Codes`)
    (if (`KismetStringLibrary.EqualEqual_StrStr` _array_element (`self.KonamiCodeSequence`))
      (set `self.KonamiCodeSequence` "")
      (`self.Execute Code` _array_index)
      (break)
      (else
        (`KismetSystemLibrary.RetriggerableDelay` 1.0)
        (set `self.KonamiCodeSequence` "")))))

(event `InputAction|Down`
  (params (Key :type "Key Structure"))
  ;[1 1 1] Code Inputs
  (:`Pressed`
    (`self.CheckCode` "d")))

(event `InputAction|Left`
  (params (Key :type "Key Structure"))
  ;[1 1 1] Code Inputs
  (:`Pressed`
    (`self.CheckCode` "l")))

(event `Execute Code`
  (params (Index :type Integer))
  ;[1 1 1] Gets correct cheat code from the array and executes the function
  (`GameplayStatics.PlaySound2D` "/Game/GIAWSystem/Audio/secret3.secret3" 1.0 1.0 0.0 null null)
  (`KismetSystemLibrary.K2_SetTimer` self (`|GetArrayItem` (`self.Cheats`) Index) 0.1))

(event `InputAction|Right`
  (params (Key :type "Key Structure"))
  ;[1 1 1] Code Inputs
  (:`Pressed`
    (`self.CheckCode` "r")))

(event `InputAction|A`
  (params (Key :type "Key Structure"))
  ;[1 1 1] Code Inputs
  (:`Pressed`
    (`self.CheckCode` "a")))

(event `InputAction|B`
  (params (Key :type "Key Structure"))
  ;[1 1 1] Code Inputs
  (:`Pressed`
    (`self.CheckCode` "b")))

(fn `SpeedCode`
  (set `self.ShipSpeed` 1600.0))

(fn `UserConstructionScript`)