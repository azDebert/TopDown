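; Game mode for the ships game that handles the start and end screens of a match.
; StartGame adds the WBP_StartGame widget to the viewport to show the countdown and instructions.
; GameOver shows WBP_EndGame with win or lose text and a matching sound, then quits the game after a short delay.
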(event `self.StartGame`
  ;[1 1 1] Display countdown and instructions
  (bind _returnvalue (`|CreateWidget` "/Game/GIAWSystem/WBP_StartGame.WBP_StartGame_C"))
  (`UserWidget.AddToViewport` _returnvalue 0))

(event `self.GameOver`
  (params (bGameWon :type Boolean))
  ;[1 1 1] Display whether the player has won or lost at the end of the game
  (bind _returnvalue (`|CreateWidget` "/Game/GIAWSystem/WBP_EndGame.WBP_EndGame_C"))
  (`UserWidget.AddToViewport` _returnvalue 0)
  (`TextBlock.SetText` (`/Game/GIAWSystem/WBP_EndGame.FinishText` _returnvalue) (select `bool` bGameWon :`false` "You Lost" :`true` "You Won" :!type "Text"))
  (if bGameWon
    (`GameplayStatics.PlaySound2D` "/Game/GIAWSystem/Audio/you_win.you_win" 1.0 1.0 0.0 null null)
    (else
      (`GameplayStatics.PlaySound2D` "/Game/GIAWSystem/Audio/you_lose.you_lose" 1.0 1.0 0.0 null null)))
  (`KismetSystemLibrary.Delay` 3.0)
  (`KismetSystemLibrary.QuitGame` null "Quit"))

(fn `UserConstructionScript`)